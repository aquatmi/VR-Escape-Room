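; BP_VendingMachine is a vending machine that dispenses a single fuse once its button has moved far enough.
; Tick watches the Button's updated X location, stopping it and setting FuseHasBeenSpawned when the threshold is reached.
; A following tick spawns a half-scale fuse at FuseSpawnPoint, assigns its type and ID, and applies a small force to its mesh.
; A Done flag prevents repeat dispensing.
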(event `self.ReceiveTick`
  (params (DeltaSeconds :type "Float (single-precision)"))
  (bind _updatedlocation_x (`KismetMathLibrary.BreakVector` (`/Game/VR_Essential_Kit/Blueprints/BP_InteractableActor.UpdatedLocation` (`self.button`))))
  (if (`self.done`)
    _
    (elif (`self.FuseHasBeenSpawned`)
      (bind _returnvalue (`|SpawnActorFromClass` (`GameplayStatics.GetObjectClass` (`self.Fuse`)) (`KismetMathLibrary.MakeTransform` (`SceneComponent.K2_GetComponentLocation` (`self.FuseSpawnPoint`)) (struct) (0.5 0.5 0.5)) "Undefined" "OverrideRootScale" null null))
      (`/Game/VR_Essential_Kit/Blueprints/BP_Fuse.setType` _returnvalue "NewEnumerator2" 1 null)
      (`PrimitiveComponent.AddForce` (`StaticMeshActor.StaticMeshComponent` _returnvalue) (-10.0 0.0 0.0) "None" false)
      (set `self.done` true)
      (`/Game/VR_Essential_Kit/Blueprints/BP_InteractableActor.Stop` (`self.button`))
      (elif (>= _updatedlocation_x 1.0)
        (set `self.FuseHasBeenSpawned` true)
        (`/Game/VR_Essential_Kit/Blueprints/BP_InteractableActor.Stop` (`self.button`))))))

(fn `UserConstructionScript`
  (set `self.FuseHasBeenSpawned` false))