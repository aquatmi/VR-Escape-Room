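; CheckFuses is a fuse puzzle checker that switches a text display to a green "OPEN" once all required fuses are in their correct slots.
; Each tick it recounts the unlocked entries in ConnectedSlots, treating an unlocked slot as a correctly placed fuse.
; The construction script fixes the required total at two.
; The match is tested before recounting, so the display updates a tick later and the solved state latches.
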(event `self.ReceiveTick`
  (params (DeltaSeconds :type "Float (single-precision)"))
  (bind _textrender (`self.TextRender`))
  ;[1 1 1] if in previous tick, all fuses were in correct slots
  (if (== (`self.totalFuses`) (`self.connectedFuses`))
    (`TextRenderComponent.K2_SetText` _textrender (`KismetTextLibrary.Conv_StringToText` "OPEN"))
    (`TextRenderComponent.SetTextRenderColor` _textrender (`KismetMathLibrary.Conv_LinearColorToColor` (`KismetMathLibrary.MakeColor` 5.0 255.0 20.0)))
    (else
      (set `self.connectedFuses` 0)
      (for _array_element (`self.ConnectedSlots`)
        ;[1 1 1] unlocked when correct fuse added
        (if (not (`/Game/VR_Essential_Kit/Blueprints/BP_Slot.Locked` _array_element))
          (set `self.connectedFuses` (+ (`self.connectedFuses`) 1)))))))

(fn `UserConstructionScript`
  (set `self.totalFuses` 2)
  (set `self.connectedFuses` 0))