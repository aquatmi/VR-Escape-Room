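; BP_PickupObject_VendingFuse is a fuse pickup, presumably dispensed by a vending machine, that stays hidden until a linked button is pressed.
; The construction script hides the mesh, and Tick polls the Button, cast to BP_InteractableActor, until its UpdatedLocation X reaches a threshold.
; Once spawned, every Tick re-enables physics and visibility, stops the Button, and applies a small constant push along negative X.
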(event `self.ReceiveTick`
  (params (DeltaSeconds :type "Float (single-precision)"))
  (bind _staticmeshcomponent (`self.StaticMeshComponent`))
  (if (`self.spawned`)
    (`PrimitiveComponent.SetSimulatePhysics` _staticmeshcomponent true)
    (`SceneComponent.SetVisibility` _staticmeshcomponent true true)
    (`/Game/BluePrints/BP_InteractableActor.Stop` (`self.button`))
    (`PrimitiveComponent.AddForce` _staticmeshcomponent (-10.0 0.0 0.0) "None" false)
    (else
      (bind _asbp_interactable_actor (cast `/Game/BluePrints/BP_InteractableActor` (`self.button`)))
      (bind _updatedlocation_x (`KismetMathLibrary.BreakVector` (`/Game/BluePrints/BP_InteractableActor.UpdatedLocation` _asbp_interactable_actor)))
      (if (>= _updatedlocation_x 1.0)
        (set `self.spawned` true)))))

(fn `UserConstructionScript`
  (bind _output_get (set `self.spawned` false))
  (`SceneComponent.SetVisibility` (`self.StaticMeshComponent`) _output_get true)
  (`parent.UserConstructionScript`))