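; Fuse box Blueprint for a puzzle where adding all three fuses triggers the win.
; On BeginPlay it moves the three referenced fuse slot actors to its fuse location components.
; Tick polls their Locked flags and, while all are false, sets the text render to "OPEN" and calls Win every frame.
; Win only calls FadeToBlack, which is empty.
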(event `self.ReceiveBeginPlay`
  ;[1 1 1] Move Fuse Slots into Position
  (`SceneComponent.K2_SetWorldLocation` (`Actor.RootComponent` (`self.Fuse1`)) (`SceneComponent.K2_GetComponentLocation` (`self.FuseLocation1`)) false false)
  (`SceneComponent.K2_SetWorldLocation` (`Actor.RootComponent` (`self.Fuse2`)) (`SceneComponent.K2_GetComponentLocation` (`self.FuseLocation2`)) false false)
  (`SceneComponent.K2_SetWorldLocation` (`Actor.RootComponent` (`self.Fuse3`)) (`SceneComponent.K2_GetComponentLocation` (`self.FuseLocation3`)) false false))

(event `self.ReceiveTick`
  (params (DeltaSeconds :type "Float (single-precision)"))
  ;[1 1 1] IF ALL FUSES ADDED
  (if (and (not (`/Game/BluePrints/Parents/BP_Slot.Locked` (`self.Fuse1`))) (not (`/Game/BluePrints/Parents/BP_Slot.Locked` (`self.Fuse2`))) (not (`/Game/BluePrints/Parents/BP_Slot.Locked` (`self.Fuse3`))))
    (`TextRenderComponent.K2_SetText` (`self.TextRender`) (`KismetTextLibrary.Conv_StringToText` "OPEN"))
    (`self.win`)))

(fn `fade to black`)

(fn `UserConstructionScript`)

(fn `win`
  (`self.fade to black`))