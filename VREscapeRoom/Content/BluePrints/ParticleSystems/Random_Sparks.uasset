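; Random_Sparks is an actor that emits occasional small spark bursts with a quiet fuse spark sound at its location.
; Each Tick it rolls a random float between the time since the last spark and 100, firing when the roll passes 99.5.
; A burst resets the timer and otherwise delta time accumulates, so the chance of a spark rises the longer none has fired.
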(event `self.ReceiveBeginPlay`)

(event `self.ReceiveTick`
  (params (DeltaSeconds :type "Float (single-precision)"))
  (bind _timesincelastspark (`self.timeSinceLastSpark`))
  (bind _returnvalue (`SceneComponent.K2_GetComponentLocation` (`self.DefaultSceneRoot`)))
  (if (> (`KismetMathLibrary.RandomFloatInRange` _timesincelastspark 100.0) 99.5)
    (`GameplayStatics.SpawnEmitterAtLocation` "/Game/BluePrints/ParticleSystems/Part_Sparks_Small.Part_Sparks_Small" _returnvalue)
    (`GameplayStatics.SpawnSoundAtLocation` "/Game/Audio/Snd_FuseSpark_Cue.Snd_FuseSpark_Cue" _returnvalue (struct) 0.2 1.0 0.0 null null)
    (set `self.timeSinceLastSpark` 0.0)
    (else
      (set `self.timeSinceLastSpark` (+ DeltaSeconds _timesincelastspark)))))

(fn `UserConstructionScript`)